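; BP_BenchTrigger is a trigger volume that marks when the player character is within sitting range of a bench.
; Overlapping its Box sets BenchSit on BP_ThirdPersonCharacter, and leaving the Box clears it.
; On entry it also adds a WBP_SitPropmpt widget to the viewport and removes it after a short fixed delay, independent of the overlap ending.
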(event `self.Box.OnComponentBeginOverlap`
  (params (OverlappedComponent :type "PrimitiveComponent Object Reference") (OtherActor :type "Actor Object Reference") (OtherComp :type "PrimitiveComponent Object Reference") (OtherBodyIndex :type Integer) (bFromSweep :type Boolean) (SweepResult :type "HitResult Structure (by ref)"))
  (bind _asbp_third_person_character (cast `/Game/ThirdPerson/Blueprints/BP_ThirdPersonCharacter` OtherActor))
  (`|ExecutionSequence`
    (:`then_0`
      (set `/Game/ThirdPerson/Blueprints/BP_ThirdPersonCharacter.BenchSit?` true _asbp_third_person_character))
    (:`then_1`
      (bind _returnvalue (`|CreateWidget` "/Game/UI/WBP_SitPropmpt.WBP_SitPropmpt_C"))
      (bind _output_get (set `self.SitHud` _returnvalue))
      (`UserWidget.AddToViewport` _output_get 0)
      (`KismetSystemLibrary.Delay` 1.0)
      (`Widget.RemoveFromParent` (`self.SitHud`)))))

(event `self.Box.OnComponentEndOverlap`
  (params (OverlappedComponent :type "PrimitiveComponent Object Reference") (OtherActor :type "Actor Object Reference") (OtherComp :type "PrimitiveComponent Object Reference") (OtherBodyIndex :type Integer))
  (bind _asbp_third_person_character (cast `/Game/ThirdPerson/Blueprints/BP_ThirdPersonCharacter` OtherActor))
  (set `/Game/ThirdPerson/Blueprints/BP_ThirdPersonCharacter.BenchSit?` false _asbp_third_person_character))

(fn `UserConstructionScript`)