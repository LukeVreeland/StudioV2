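; BP_Bow is a bow pickup actor for the third-person character.
; Its Box overlap sets BowPickup and HasBow on BP_ThirdPersonCharacter, while leaving the box clears only BowPickup.
; The PickUp event waits a tick, then runs a timeline that scales the bow mesh by its Shrink track and destroys the actor after a short delay.
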(event `/Game/BluePrints/bpi_Bow.PickUp`
  (`KismetSystemLibrary.DelayUntilNextTick`)
  (`|ExecutionSequence`
    (:`then_0`
      (bind (_direction _shrink) (`Timeline|Timeline`)
        (:`Update`
          (`SceneComponent.SetWorldScale3D` (`self.Bow`) (`KismetMathLibrary.Conv_DoubleToVector` (`KismetMathLibrary.Lerp` 0.0 1.0 _shrink))))))
    (:`then_1`
      (`KismetSystemLibrary.Delay` 0.2)
      (`self.K2_DestroyActor`))))

(event `self.Box.OnComponentBeginOverlap`
  (params (OverlappedComponent :type "PrimitiveComponent Object Reference") (OtherActor :type "Actor Object Reference") (OtherComp :type "PrimitiveComponent Object Reference") (OtherBodyIndex :type Integer) (bFromSweep :type Boolean) (SweepResult :type "HitResult Structure (by ref)"))
  (bind _asbp_third_person_character (cast `/Game/ThirdPerson/Blueprints/BP_ThirdPersonCharacter` OtherActor))
  (set `/Game/ThirdPerson/Blueprints/BP_ThirdPersonCharacter.bowPickup?` true _asbp_third_person_character)
  (set `/Game/ThirdPerson/Blueprints/BP_ThirdPersonCharacter.Has Bow?` true _asbp_third_person_character))

(event `self.Box.OnComponentEndOverlap`
  (params (OverlappedComponent :type "PrimitiveComponent Object Reference") (OtherActor :type "Actor Object Reference") (OtherComp :type "PrimitiveComponent Object Reference") (OtherBodyIndex :type Integer))
  (bind _asbp_third_person_character (cast `/Game/ThirdPerson/Blueprints/BP_ThirdPersonCharacter` OtherActor))
  (set `/Game/ThirdPerson/Blueprints/BP_ThirdPersonCharacter.bowPickup?` false _asbp_third_person_character))

(fn `UserConstructionScript`)