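; Controller Blueprint for switching possession among the BP_ThirdPersonCharacter actors in the level.
; BeginPlay stores every such character in a roster and records player 0's pawn as the current character.
; Tab calls NextCharacter, which is named for cycling but always possesses roster index 0, because its select is fixed to false and the next-index validity check is unconnected.
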(event `self.ReceiveBeginPlay`
  (bind _outactors (`GameplayStatics.GetAllActorsOfClass` "/Game/ThirdPerson/Blueprints/BP_ThirdPersonCharacter.BP_ThirdPersonCharacter_C"))
  (set `self.Character Roster` _outactors)
  (bind _asbp_third_person_character (cast `/Game/ThirdPerson/Blueprints/BP_ThirdPersonCharacter` (`GameplayStatics.GetPlayerCharacter` 0)))
  (set `self.Current Character` _asbp_third_person_character))

(event `Key|Tab`
  (params (Key :type "Key Structure"))
  (:`Pressed`
    (`self.Next Character`)))

(fn `Next Character`
  (locals (Local_Index :type Integer))
  (bind _returnvalue (`KismetArrayLibrary.Array_Find` (`self.Character Roster`) (`self.Current Character`)))
  (set `local.Local_Index` _returnvalue)
  (bind _output_get (set `local.Local_Index` (`KismetMathLibrary.SelectInt` (+ _returnvalue 1))))
  (bind _output_get_2 (set `self.Current Character` (`|GetArrayItem` (`self.Character Roster`) _output_get)))
  (`self.Possess` _output_get_2))

(fn `UserConstructionScript`)