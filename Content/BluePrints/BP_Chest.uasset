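; Interactable chest that a player holding a key opens with E to receive a sword.
; Box overlap toggles input and caches the third-person character for the key check.
; With a key, a one-time timeline rotates the lid, then delays trigger a Niagara effect, remove the chest components and spawn BP_Sword at the Arrow.
; Without one, a WBP_Chest widget shows briefly, throttled by a resetting DoOnce.
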(event `Key|E`
  (params (Key :type "Key Structure"))
  (bind _returnvalue_location (`KismetMathLibrary.BreakTransform` (`SceneComponent.K2_GetComponentToWorld` (`self.Arrow`))))
  (:`Pressed`
    (`|ExecutionSequence`
      (:`then_0`
        (if (`/Game/ThirdPerson/Blueprints/BP_ThirdPersonCharacter.Has Key?` (stale `self.Box.OnComponentBeginOverlap` _asbp_third_person_character))
          (`/Engine/EditorBlueprintResources/StandardMacros.DoOnce` false
            (:`Completed`
              (`|ExecutionSequence`
                (:`then_0`
                  (bind (_direction _chestfloat) (`Timeline|Open Chest` :!via `PlayFromStart`)
                    (:`Update`
                      (`SceneComponent.K2_SetRelativeRotation` (`self.ChestTop`) (`KismetMathLibrary.MakeRotator` (`KismetMathLibrary.Lerp` 0.0 60.0 _chestfloat) 0.0 180.0) false false)
                      (`|ExecutionSequence`
                        (:`then_0`
                          (`KismetSystemLibrary.Delay` 2.5)
                          (`|SpawnActorFromClass` "/Game/BluePrints/BP_Sword.BP_Sword_C" (`KismetMathLibrary.MakeTransform` _returnvalue_location) "Undefined" "MultiplyWithRoot" null null))
                        (:`then_1`
                          (`KismetSystemLibrary.Delay` 2.4)
                          (bind _returnvalue (`AddComponent|NODE_AddNiagaraComponent-0`))
                          (`ActorComponent.Activate` _returnvalue false))
                        (:`then_2`
                          (`|ExecutionSequence`
                            (:`then_0`
                              (`KismetSystemLibrary.Delay` 2.4)
                              (`ActorComponent.K2_DestroyComponent` (`self.Chest Bottom`)))
                            (:`then_1`
                              (`KismetSystemLibrary.Delay` 2.4)
                              (`ActorComponent.K2_DestroyComponent` (`self.ChestTop`)))
                            (:`then_2`
                              (`KismetSystemLibrary.Delay` 2.4)
                              (`ActorComponent.K2_DestroyComponent` (`self.Box`))))))))))))
          (else
            (`/Engine/EditorBlueprintResources/StandardMacros.DoOnce` false :!label _label
              (:`Completed`
                (bind _returnvalue_2 (`|CreateWidget` "/Game/UI/WBP_Chest.WBP_Chest_C"))
                (bind _output_get (set `self.Chest Hud` _returnvalue_2))
                (`UserWidget.AddToViewport` _output_get 0)
                (`KismetSystemLibrary.Delay` 1.0)
                (`Widget.RemoveFromParent` (`self.Chest Hud`)))))))
      (:`then_1`
        (`KismetSystemLibrary.Delay` 1.0)
        (goto _label :!via `Reset`)))))

(event `self.Box.OnComponentBeginOverlap`
  (params (OverlappedComponent :type "PrimitiveComponent Object Reference") (OtherActor :type "Actor Object Reference") (OtherComp :type "PrimitiveComponent Object Reference") (OtherBodyIndex :type Integer) (bFromSweep :type Boolean) (SweepResult :type "HitResult Structure (by ref)"))
  (bind _asbp_third_person_character (cast `/Game/ThirdPerson/Blueprints/BP_ThirdPersonCharacter` OtherActor))
  (`self.EnableInput` (`GameplayStatics.GetPlayerController` 0)))

(event `self.Box.OnComponentEndOverlap`
  (params (OverlappedComponent :type "PrimitiveComponent Object Reference") (OtherActor :type "Actor Object Reference") (OtherComp :type "PrimitiveComponent Object Reference") (OtherBodyIndex :type Integer))
  (cast `/Game/ThirdPerson/Blueprints/BP_ThirdPersonCharacter` OtherActor)
  (`self.DisableInput` (`GameplayStatics.GetPlayerController` 0)))

(fn `UserConstructionScript`)