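; BP_Sword is a sword pickup for BP_ThirdPersonCharacter, with its mesh set from the SModel variable in the construction script.
; Entering its Box sets the character's SwordPickUp and HasSword flags for animation, while leaving clears only SwordPickUp.
; The PickUp event waits a tick, then shrinks the actor with a timeline and destroys it after a short delay.
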(event `/Game/BluePrints/bpi_Sword.Pick Up`
  (`KismetSystemLibrary.DelayUntilNextTick`)
  (`|ExecutionSequence`
    (:`then_0`
      (bind (_direction _shrink) (`Timeline|Shrink`)
        (:`Update`
          (`SceneComponent.SetWorldScale3D` (`self.DefaultSceneRoot`) (`KismetMathLibrary.Conv_DoubleToVector` (`KismetMathLibrary.Lerp` 1.0 0.0 _shrink))))))
    (:`then_1`
      (`KismetSystemLibrary.Delay` 0.2)
      (`self.K2_DestroyActor`))))

(event `self.Box.OnComponentBeginOverlap`
  (params (OverlappedComponent :type "PrimitiveComponent Object Reference") (OtherActor :type "Actor Object Reference") (OtherComp :type "PrimitiveComponent Object Reference") (OtherBodyIndex :type Integer) (bFromSweep :type Boolean) (SweepResult :type "HitResult Structure (by ref)"))
  ; For animation
  (bind _asbp_third_person_character (cast `/Game/ThirdPerson/Blueprints/BP_ThirdPersonCharacter` OtherActor))
  (set `/Game/ThirdPerson/Blueprints/BP_ThirdPersonCharacter.SwordPickUp?` true _asbp_third_person_character)
  (set `/Game/ThirdPerson/Blueprints/BP_ThirdPersonCharacter.HasSword?` true _asbp_third_person_character))

(event `self.Box.OnComponentEndOverlap`
  (params (OverlappedComponent :type "PrimitiveComponent Object Reference") (OtherActor :type "Actor Object Reference") (OtherComp :type "PrimitiveComponent Object Reference") (OtherBodyIndex :type Integer))
  ; For animation
  (bind _asbp_third_person_character (cast `/Game/ThirdPerson/Blueprints/BP_ThirdPersonCharacter` OtherActor))
  (set `/Game/ThirdPerson/Blueprints/BP_ThirdPersonCharacter.SwordPickUp?` false _asbp_third_person_character))

(fn `UserConstructionScript`
  (`StaticMeshComponent.SetStaticMesh` (`self.Sword`) (`self.SModel`)))