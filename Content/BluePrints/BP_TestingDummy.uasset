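; Testing dummy actor that takes damage and shows a health bar and damage numbers through widget components.
; Tick sets the bar from CurrentHealth over MaxHealth and turns it toward the player camera.
; AnyDamage sets health to MaxHealth minus that hit, so damage does not accumulate, then shows the amount on a camera-facing indicator.
; The actor is destroyed only when damage arrives with health already at or below zero.
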(event `self.ReceiveTick`
  (params (DeltaSeconds :type "Float (single-precision)"))
  (bind _healthbar (`self.healthBar`))
  (bind _aswbp_enemy_health_bar (cast `/Game/UI/WBP_EnemyHealthBar` (`WidgetComponent.GetWidget` (`self.healthBar`))))
  (`ProgressBar.SetPercent` (`/Game/UI/WBP_EnemyHealthBar.Healthbar` _aswbp_enemy_health_bar) (/ (`self.currentHealth`) (`self.maxHealth`)))
  (`SceneComponent.K2_SetWorldRotation` _healthbar (`KismetMathLibrary.FindLookAtRotation` (`SceneComponent.K2_GetComponentLocation` _healthbar) (`SceneComponent.K2_GetComponentLocation` (`PlayerCameraManager.TransformComponent` (`GameplayStatics.GetPlayerCameraManager` 0)))) false false))

(event `self.ReceiveAnyDamage`
  (params (Damage :type "Float (single-precision)") (DamageType :type "DamageType Object Reference") (InstigatedBy :type "Controller Object Reference") (DamageCauser :type "Actor Object Reference"))
  (bind _damageindictator (`self.damageIndictator`))
  (if (> (`self.currentHealth`) 0)
    (set `self.currentHealth` (`KismetMathLibrary.FTrunc` (- (`self.maxHealth`) Damage)))
    (bind _aswbp_damage_numbers (cast `/Game/UI/WBP_DamageNumbers` (`WidgetComponent.GetWidget` (`self.damageIndictator`))))
    (`/Game/UI/WBP_DamageNumbers.appliedDamage` _aswbp_damage_numbers (`KismetTextLibrary.Conv_DoubleToText` Damage "HalfToEven"))
    (`SceneComponent.K2_SetWorldRotation` _damageindictator (`KismetMathLibrary.FindLookAtRotation` (`SceneComponent.K2_GetComponentLocation` _damageindictator) (`SceneComponent.K2_GetComponentLocation` (`PlayerCameraManager.TransformComponent` (`GameplayStatics.GetPlayerCameraManager` 0)))) false false)
    (else
      (`self.K2_DestroyActor`))))

(fn `UserConstructionScript`)