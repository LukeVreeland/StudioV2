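; Corridor trigger actor that shows the WB_Corridor1 notification widget when the third-person character enters its Box.
; Box overlaps set and clear the character's InWidgetBox flag; entry also creates the widget, adds it to the viewport and plays its animation after a short delay.
; A DoOnce limits repeats, and a delayed second Sequence branch resets it, even when the overlapping actor is not the character.
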(event `self.Box.OnComponentBeginOverlap`
  (params (OverlappedComponent :type "PrimitiveComponent Object Reference") (OtherActor :type "Actor Object Reference") (OtherComp :type "PrimitiveComponent Object Reference") (OtherBodyIndex :type Integer) (bFromSweep :type Boolean) (SweepResult :type "HitResult Structure (by ref)"))
  (`|ExecutionSequence`
    (:`then_0`
      (bind _asbp_third_person_character (cast `/Game/ThirdPerson/Blueprints/BP_ThirdPersonCharacter` OtherActor))
      (set `/Game/ThirdPerson/Blueprints/BP_ThirdPersonCharacter.In Widget Box?` true _asbp_third_person_character)
      (`/Engine/EditorBlueprintResources/StandardMacros.DoOnce` false :!label _label
        (:`Completed`
          (bind _returnvalue (`|CreateWidget` "/Game/UI/CorridorWidgets/WB_Corridor1.WB_Corridor1_C"))
          (`UserWidget.AddToViewport` _returnvalue 0)
          (`KismetSystemLibrary.Delay` 0.3)
          (`/Game/UI/CorridorWidgets/WB_Corridor1.Play Notification Animation` _returnvalue))))
    (:`then_1`
      (`KismetSystemLibrary.Delay` 6.0)
      (goto _label :!via `Reset`))))

(event `self.Box.OnComponentEndOverlap`
  (params (OverlappedComponent :type "PrimitiveComponent Object Reference") (OtherActor :type "Actor Object Reference") (OtherComp :type "PrimitiveComponent Object Reference") (OtherBodyIndex :type Integer))
  (bind _asbp_third_person_character (cast `/Game/ThirdPerson/Blueprints/BP_ThirdPersonCharacter` OtherActor))
  (set `/Game/ThirdPerson/Blueprints/BP_ThirdPersonCharacter.In Widget Box?` false _asbp_third_person_character))

(fn `UserConstructionScript`)